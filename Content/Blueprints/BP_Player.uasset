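; BP_Player is the player character, with on-screen HP, a death montage that ends in destruction, and shooting at monsters.
; Fire traces from both weapon sockets toward a point deprojected from screen center, but only the right-hand trace damages BP_Monster.
; AnyDamage lowers HP until it is negative; only a later hit starts death.
; Helper functions provide a launch jump, walk speed switching and bomb knockback away from a hit location.
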(event `self.ReceiveTick`
  (params (DeltaSeconds :type "Float (single-precision)"))
  (`KismetSystemLibrary.PrintText` (`|FormatText` "Player HP : { 0 }" (stale `self.ReceiveAnyDamage` _output_get)) true true (struct :`G` 0.66 :`B` 1.0 :`A` 1.0) 0.0 :!label _label))

(event `self.ReceiveAnyDamage`
  (params (Damage :type "Float (single-precision)") (DamageType :type "DamageType Object Reference") (InstigatedBy :type "Controller Object Reference") (DamageCauser :type "Actor Object Reference"))
  (if (>= (`self.HP`) 0)
    (bind _output_get (set `self.HP` (- (`self.HP`) Damage)))
    (goto _label)
    (else
      (`|PlayMontage` (`self.Mesh`) "/Game/Animations/AM_PlayerDeath.AM_PlayerDeath"
        (:`OnCompleted`
          (`self.K2_DestroyActor`))))))

(fn `Bomb`
  (params (HitLocation :type "Vector Structure"))
  (locals (NewLocalVar :type "Vector Structure") (NewLocalVar_0 :type "Vector Structure"))
  (`self.LaunchCharacter` (+ (* (`KismetMathLibrary.Normal` (- (`self.K2_GetActorLocation`) HitLocation)) 1500.0) (0.0 0.0 300.0)) true))

(fn `Fire`
  (bind (_returnvalue_x _returnvalue_y) (`KismetMathLibrary.BreakVector2D` (`WidgetLayoutLibrary.GetViewportSize`)))
  (bind (_worldposition _worlddirection) (`GameplayStatics.DeprojectScreenToWorld` (`GameplayStatics.GetPlayerController` 0) (`KismetMathLibrary.MakeVector2D` (/ _returnvalue_x 2.0) (/ _returnvalue_y 2.0))))
  (`self.PlayAnimMontage` "/Game/Animations/AM_Fire.AM_Fire")
  (bind _outhit (`KismetSystemLibrary.LineTraceSingle` :`Start` (`SceneComponent.GetSocketLocation` (`self.Mesh`) "WeaponSocket_R") :`End` (+ _worldposition (* _worlddirection 5000.0)) :`TraceChannel` "TraceTypeQuery1" :`DrawDebugType` "ForDuration"))
  (bind (_bblockinghit _binitialoverlap _time _distance _location _impactpoint _normal _impactnormal _physmat _hitactor _hitcomponent _hitbonename _bonename _hititem _elementindex _faceindex _tracestart _traceend) (`GameplayStatics.BreakHitResult` _outhit))
  (`KismetSystemLibrary.LineTraceSingle` :`Start` (`SceneComponent.GetSocketLocation` (`self.Mesh`) "WeaponSocket_L") :`End` _traceend :`TraceChannel` "TraceTypeQuery1" :`DrawDebugType` "ForDuration")
  (bind _asbp_monster (cast `/Game/Blueprints/BP_Monster` _hitactor))
  (`GameplayStatics.ApplyDamage` _asbp_monster 3.0))

(fn `GetOriginSpeed`
  (set `CharacterMovementComponent.MaxWalkSpeed` (`self.BaseSpeed`) (`self.CharacterMovement`)))

(fn `GetSlowed`
  (set `CharacterMovementComponent.MaxWalkSpeed` (`self.CurrentSpeed`) (`self.CharacterMovement`)))

(fn `SuperJump`
  (`self.LaunchCharacter` (0.0 0.0 1300.0)))

(fn `UserConstructionScript`)