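; BP_WoodObstacle is a moving wooden obstacle that damages the player on contact.
; Each tick it accumulates running time and uses a sine wave, scaled by move speed and distance, to oscillate around a start location along the Wood component's forward vector, without sweeping.
; When Wood registers a hit with BP_Player, it applies fixed damage and prints a red on-screen message.
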(event `self.ReceiveTick`
  (params (DeltaSeconds :type "Float (single-precision)"))
  (bind _output_get (set `self.RunningTime` (+ DeltaSeconds (`self.RunningTime`))))
  (`self.K2_SetActorLocation` (+ (`self.StartLocation`) (* (`SceneComponent.GetForwardVector` (`self.Wood`)) (* (`KismetMathLibrary.Sin` (* _output_get (`self.MoveSpeed`))) (`self.MoveDistance`))))))

(event `self.Wood.OnComponentHit`
  (params (HitComponent :type "PrimitiveComponent Object Reference") (OtherActor :type "Actor Object Reference") (OtherComp :type "PrimitiveComponent Object Reference") (NormalImpulse :type "Vector Structure") (Hit :type "HitResult Structure (by ref)"))
  (bind _asbp_player (cast `/Game/Blueprints/BP_Player` OtherActor))
  (`GameplayStatics.ApplyDamage` _asbp_player 5.0)
  (`KismetSystemLibrary.PrintString` "Player Damaged -5!" true true (struct :`R` 0.994792 :`A` 1.0) 12.0))

(fn `UserConstructionScript`)