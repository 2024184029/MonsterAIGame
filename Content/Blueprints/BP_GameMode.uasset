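; Game mode for a timed round with monsters and wood obstacles.
; On BeginPlay it spawns ten BP_Monster actors at random reachable navmesh points around its location.
; Tick accumulates running time and prints it until the limit, then prints "Time Over!" and destroys all monsters and wood obstacles every frame.
; A CheckAndSpawn call is disconnected, with a note that a runtime error needs fixing.
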(event `self.ReceiveBeginPlay`
  (for _ (range 10)
    (`|SpawnActorFromClass` "/Game/Blueprints/BP_Monster.BP_Monster_C" (`KismetMathLibrary.MakeTransform` (`NavigationSystemV1.K2_GetRandomReachablePointInRadius` (`self.K2_GetActorLocation`) 3000.0 null null)) "Undefined" "MultiplyWithRoot" null null)))

(event `self.ReceiveTick`
  (params (DeltaSeconds :type "Float (single-precision)"))
  (bind _output_get (set `self.RunningTime` (+ DeltaSeconds (`self.RunningTime`))))
  (if (< _output_get (`self.LimitTime`))
    (`KismetSystemLibrary.PrintText` (`|FormatText` "Time Limit - 03:00 \nRunning Time - 0{ 0 }m { 1 }" (mod (`KismetMathLibrary.FTrunc` _output_get) 60) _) true true (struct :`G` 0.66 :`B` 1.0 :`A` 1.0) 0.0)
    (else
      (`KismetSystemLibrary.PrintString` "Time Over!" true true (struct :`G` 0.66 :`B` 1.0 :`A` 1.0) 0.0)
      (bind _outactors (`GameplayStatics.GetAllActorsOfClass` "/Game/Blueprints/BP_WoodObstacle.BP_WoodObstacle_C"))
      (`self.K2_DestroyActor` _outactors)
      (bind _outactors_2 (`GameplayStatics.GetAllActorsOfClass` "/Game/Blueprints/BP_Monster.BP_Monster_C"))
      (`self.K2_DestroyActor` _outactors_2))))

(fn `UserConstructionScript`)