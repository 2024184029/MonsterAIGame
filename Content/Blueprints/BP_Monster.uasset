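; BP_Monster is an enemy character with a randomized walk speed that can take damage and attack the player.
; BeginPlay rolls the speed into CharacterMovement, while AnyDamage subtracts and prints HP, destroying the monster only on a hit received once HP is already depleted.
; AttackHit, not called within this Blueprint, damages BP_Player if within Distance and prints debug messages for hits or failed casts.
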(event `self.ReceiveBeginPlay`
  (bind _output_get (set `self.Speed` (`KismetMathLibrary.RandomFloatInRange` 100.0 400.0)))
  (set `CharacterMovementComponent.MaxWalkSpeed` _output_get (`self.CharacterMovement`)))

(event `self.ReceiveAnyDamage`
  (params (Damage :type "Float (single-precision)") (DamageType :type "DamageType Object Reference") (InstigatedBy :type "Controller Object Reference") (DamageCauser :type "Actor Object Reference"))
  (if (> (`self.HP`) 0)
    (bind _output_get (set `self.HP` (- (`self.HP`) Damage)))
    (`KismetSystemLibrary.PrintText` (`|FormatText` "Monster HP : { 0 }" _output_get) true true (struct :`G` 0.66 :`B` 1.0 :`A` 1.0) 10.0)
    (else
      (`self.K2_DestroyActor`))))

(fn `AttackHit`
  (bind _asbp_player (cast `/Game/Blueprints/BP_Player` (`GameplayStatics.GetPlayerCharacter` 0))
    (:`then`
      (if (< (`KismetMathLibrary.VSize` (- (`self.K2_GetActorLocation`) (`self.K2_GetActorLocation` (`GameplayStatics.GetPlayerCharacter` 0)))) (`self.Distance`))
        (`GameplayStatics.ApplyDamage` _asbp_player 1.0)
        (`KismetSystemLibrary.PrintString` "공격 당했습니다!" true true (struct :`G` 0.66 :`B` 1.0 :`A` 1.0) 5.0)))
    (:`CastFailed`
      (`KismetSystemLibrary.PrintString` "캐스팅 안 됨" true true (struct :`G` 0.66 :`B` 1.0 :`A` 1.0) 100.0))))

(fn `UserConstructionScript`)