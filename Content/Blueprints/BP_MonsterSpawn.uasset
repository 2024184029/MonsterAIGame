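; BP_MonsterSpawn is a spawner actor that populates the area around itself with BP_Monster actors at random reachable navmesh points.
; BeginPlay spawns an initial batch without incrementing CurrentMonster.
; Tick calls CheckAndSpawn, which, while CurrentMonster is below MaxMonster, waits a random Delay, spawns a monster, increments the count and calls itself again.
; The file never decrements CurrentMonster, so removed monsters are not replaced by this logic alone.
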(event `CheckAndSpawn`
  (if (< (`self.CurrentMonster`) (`self.MaxMonster`))
    (bind _output_get (set `self.RandomTime` (`KismetMathLibrary.RandomFloatInRange` 1.0 5.0)))
    (`KismetSystemLibrary.Delay` _output_get)
    (`|SpawnActorFromClass` "/Game/Blueprints/BP_Monster.BP_Monster_C" (`KismetMathLibrary.MakeTransform` (`NavigationSystemV1.K2_GetRandomReachablePointInRadius` (`self.K2_GetActorLocation`) 3000.0 null null)) "Undefined" "MultiplyWithRoot" null null)
    (set `self.CurrentMonster` (+ (`self.CurrentMonster`) 1))
    (`self.CheckAndSpawn`)))

(event `self.ReceiveBeginPlay`
  (for _ (range 10)
    (`|SpawnActorFromClass` "/Game/Blueprints/BP_Monster.BP_Monster_C" (`KismetMathLibrary.MakeTransform` (`NavigationSystemV1.K2_GetRandomReachablePointInRadius` (`self.K2_GetActorLocation`) 3000.0 null null)) "Undefined" "MultiplyWithRoot" null null)))

(event `self.ReceiveTick`
  (params (DeltaSeconds :type "Float (single-precision)"))
  (`self.CheckAndSpawn`))

(fn `UserConstructionScript`)