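; Behavior tree service that finds the player and flags it as a chase target when it is near the AI's pawn.
; On activation it waits briefly, then caches the first BP_Player actor in the level.
; Each service tick compares the distance to the controlled pawn, setting the Player blackboard key within 5 m and clearing it otherwise.
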(event `self.ReceiveActivationAI`
  (params (OwnerController :type "AIController Object Reference") (ControlledPawn :type "Pawn Object Reference"))
  ; 플레이어 인스턴스 가져와서 연결시키기
  (`KismetSystemLibrary.Delay` 0.2)
  (bind _returnvalue (`GameplayStatics.GetActorOfClass` "/Game/Blueprints/BP_Player.BP_Player_C"))
  (set `self.BPPlayer` _returnvalue))

(event `self.ReceiveTickAI`
  (params (OwnerController :type "AIController Object Reference") (ControlledPawn :type "Pawn Object Reference") (DeltaSeconds :type "Float (single-precision)"))
  (bind _bpplayer (`self.BPPlayer`))
  (`/Engine/EditorBlueprintResources/StandardMacros.IsValid` _bpplayer
    (:`Is Valid`
      (if (<= (`KismetMathLibrary.VSize` (- (`Actor.K2_GetActorLocation` _bpplayer) (`Actor.K2_GetActorLocation` ControlledPawn))) 500.0)
        ; 추격
        (`BTFunctionLibrary.SetBlackboardValueAsObject` (`self.Player`) (`self.BPPlayer`))
        (else
          (`BTFunctionLibrary.SetBlackboardValueAsObject` (`self.Player`)))))))