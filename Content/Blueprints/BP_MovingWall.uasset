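; BP_MovingWall is an obstacle wall that slides back and forth and damages the player on contact.
; Each Tick offsets the actor from its BeginPlay location along the wall component's right vector, using a sine of accumulated time scaled by MoveSpeed and MoveDistance, without sweeping.
; Component hits from BP_Player apply damage and print a warning, gated by a DoOnce that resets after a short delay as a cooldown.
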(event `self.ReceiveBeginPlay`
  (set `self.StartLocation` (`self.K2_GetActorLocation`)))

(event `self.ReceiveTick`
  (params (DeltaSeconds :type "Float (single-precision)"))
  (bind _output_get (set `self.RunningTime` (+ DeltaSeconds (`self.RunningTime`))))
  (`self.K2_SetActorLocation` (+ (`self.StartLocation`) (* (`SceneComponent.GetRightVector` (`self.MovingWall`)) (* (`KismetMathLibrary.Sin` (* _output_get (`self.MoveSpeed`))) (`self.MoveDistance`))))))

(event `self.MovingWall.OnComponentHit`
  (params (HitComponent :type "PrimitiveComponent Object Reference") (OtherActor :type "Actor Object Reference") (OtherComp :type "PrimitiveComponent Object Reference") (NormalImpulse :type "Vector Structure") (Hit :type "HitResult Structure (by ref)"))
  (bind _asbp_player (cast `/Game/Blueprints/BP_Player` OtherActor))
  (`/Engine/EditorBlueprintResources/StandardMacros.DoOnce` false :!label _label
    (:`Completed`
      (`GameplayStatics.ApplyDamage` _asbp_player 5.0)
      (`KismetSystemLibrary.PrintString` "벽과 부딪혔습니다 ! \n[Player Damaged -5]" true true (struct :`R` 0.994792 :`A` 1.0) 5.0)
      (`KismetSystemLibrary.Delay` 1.0)
      (goto _label :!via `Reset`))))

(fn `UserConstructionScript`)